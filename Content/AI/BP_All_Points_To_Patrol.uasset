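; Actor that gathers and orders the level's patrol points for AI patrolling.
; InitializeArrays finds every BP_Patroll_Point, bubble-sorts them ascending by their Number, and stores the first one as NextPoint.
; BeginPlay is empty, so InitializeArrays runs only when called from elsewhere; leftover debug prints are disconnected.
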(event Custom|Initialize%20Arrays
  (bind _outactors (Actor|GetAllActorsOfClass "/Game/AI/BP_Patroll_Point.BP_Patroll_Point_C"))
  (bind _output_get (Variables|Default|SetAllPoints _outactors))
  ;[0.15 0.15 0.15 0.5] Bubble sort
  (bind _index (Utilities|FlowControl|ForLoopwithBreak 0 (- (Utilities|Array|Length _output_get) 2))
    (:LoopBody
      (bind _index_2 (Utilities|FlowControl|ForLoopwithBreak 0 (- (- (Utilities|Array|Length _output_get) 2) _index))
        (:LoopBody
          (if (> (Variables|/Game/AI/BP_Patroll_Point.BP_Patroll_Point_C|GetNumber (Utilities|Array|Get(acopy) (Variables|Default|GetAllPoints) _index_2)) (Variables|/Game/AI/BP_Patroll_Point.BP_Patroll_Point_C|GetNumber (Utilities|Array|Get(acopy) (Variables|Default|GetAllPoints) (+ _index_2 1))))
            (Utilities|Array|Swap (Variables|Default|GetAllPoints) _index_2 (+ _index_2 1))))))
    (:Completed
      (Variables|Default|SetNextPoint (Utilities|Array|Get(acopy) (Variables|Default|GetAllPoints))))))

(event EventBeginPlay)

(event Collision|EventActorBeginOverlap
  (params (OtherActor :type Actor%20Object%20Reference)))

(event EventTick
  (params (DeltaSeconds :type Float%20%28single-precision%29)))

(fn ConstructionScript)